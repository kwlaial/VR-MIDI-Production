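; MIDI keyboard test Blueprint that logs incoming MIDI events on screen.
; BeginPlay creates an output controller for the default device, while a DoOnce on Tick creates an input controller for a hardcoded device ID and binds its event.
; The handler prints details of events with non-zero velocity.
; An unconnected, never-run branch sketches six-voice MetaSound playback, using note and velocity arrays to set key parameters and fire triggers.
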(event Custom|CustomEvent_0
  (params (MIDIDeviceController :type MIDI%20Device%20Controller%20Object%20Reference) (Timestamp :type Integer) (EventType :type EMIDIEventType%20Enum :default "Unknown") (Channel :type Integer) (ControlID :type Integer) (Velocity :type Integer) (RawEventType :type Integer))
  (Utilities|IsValid MIDIDeviceController
    (:Is%20Valid
      (if (!= Velocity 0)
        (Development|PrintText (Utilities|Text|FormatText "{Timestamp}: Ch{Channel} - {EventType} /ID: {ControlId}, Vel: {Velocity}" (Utilities|Text|ToText(Integer) Timestamp) (Utilities|Text|ToText(Integer) Channel) (Utilities|Text|ToText(String) (Utilities|String|ToString(Byte) EventType)) (Utilities|Text|ToText(Integer) ControlID) (Utilities|Text|ToText(Integer) Velocity)))))))

(event EventBeginPlay
  ;[1 1 1] Looking for MIDI device
  (bind _deviceid (Class|MIDIDeviceManager|GetDefaultMIDIOutputDeviceID))
  (Class|MIDIDeviceManager|CreateMIDIDeviceOutputController _deviceid))

(event Collision|EventActorBeginOverlap
  (params (OtherActor :type Actor%20Object%20Reference)))

(event EventTick
  (params (DeltaSeconds :type Float%20%28single-precision%29))
  (Utilities|FlowControl|DoOnce false
    (:Completed
      (bind _returnvalue (Class|MIDIDeviceManager|CreateMIDIDeviceController 1 1024))
      (Utilities|IsValid _returnvalue
        (:Is%20Valid
          (bind _output_get (Variables|Default|SetNewVar_0 _returnvalue)))
        (:Is%20Not%20Valid
          _))
      (Development|PrintString (Utilities|GetDisplayName _output_get) true true "(R=0.065278,G=1.000000,B=0.000000,A=1.000000)")
      (EventDispatchers|BindEventtoOnMIDIEvent _returnvalue (delegate Custom|CustomEvent_0)))))

(fn ConstructionScript)